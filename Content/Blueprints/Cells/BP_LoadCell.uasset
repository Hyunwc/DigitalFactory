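; BP_LoadCell is a load cell that operates a door and takes a vehicle body from the working AGV.
; A timeline lerps the door between closed and open relative locations, reversing to close it.
; VehicleLoadtoSpline detaches the AGV's attached vehicle, enables actor tick and snaps the vehicle to the spline's start.
; The Tick event here is empty, so this graph does not move the vehicle along the spline.
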(event EventBeginPlay)

(event Collision|EventActorBeginOverlap
  (params (OtherActor :type Actor%20Object%20Reference)))

(event EventTick
  (params (DeltaSeconds :type Float%20%28single-precision%29)))

(event EventOpenDoor
  (bind _alpha (Timeline|DoorTimeLine PlayFromStart)
    (:Update
      (Transformation|SetRelativeLocation (Variables|Default|GetDoor) (Math|Vector|Lerp(Vector) (Variables|Default|GetCloseDoorLocation) (Variables|Default|GetOpenDoorLocation) _alpha) false false))))

(event EventCloseDoor
  (bind _alpha (Timeline|DoorTimeLine Reverse)
    (:Update
      (Transformation|SetRelativeLocation (Variables|Default|GetDoor) (Math|Vector|Lerp(Vector) (Variables|Default|GetCloseDoorLocation) (Variables|Default|GetOpenDoorLocation) _alpha) false false))))

(event EventVehicleLoadtoSpline
  ;[0 0 0 0.5] 작업중인 AGV가 들고있는 차체를 디태치
  (Transformation|DetachFromActor (Variables|/Script/DigitalFactory.DFAGV|GetAttachVehicle (Variables|Default|GetWorkingAGV)) "KeepWorld" "KeepWorld" "KeepWorld")
  (Actor|Tick|SetActorTickEnabled true)
  (Transformation|SetActorLocation (Variables|/Script/DigitalFactory.DFAGV|GetAttachVehicle (Variables|Default|GetWorkingAGV)) (Spline|GetLocationatDistanceAlongSpline (Variables|Default|GetSpline) 0.0 "World") false false))

(fn ConstructionScript)