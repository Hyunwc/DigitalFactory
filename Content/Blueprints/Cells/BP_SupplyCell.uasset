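; BP_SupplyCell is a supply cell that hands a vehicle body to a working AGV and has an animated door.
; A timeline lerps the door between closed and open locations, and closing plays the same timeline in reverse.
; AttachVehicle snaps the supply vehicle to a socket on the AGV's mesh.
; On success, it sets the AGV's vehicle reference, copies the order color onto the vehicle and resets the cell data.
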(event EventBeginPlay)

(event Collision|EventActorBeginOverlap
  (params (OtherActor :type Actor%20Object%20Reference)))

(event EventTick
  (params (DeltaSeconds :type Float%20%28single-precision%29)))

(event EventOpenDoor
  (bind _alpha (Timeline|DoorTimeLine PlayFromStart)
    (:Update
      (Transformation|SetRelativeLocation (Variables|Default|GetDoor) (Math|Vector|Lerp(Vector) (Variables|Default|GetCloseDoorLocation) (Variables|Default|GetOpenDoorLocation) _alpha) false false))))

(event EventCloseDoor
  (bind _alpha (Timeline|DoorTimeLine Reverse)
    (:Update
      (Transformation|SetRelativeLocation (Variables|Default|GetDoor) (Math|Vector|Lerp(Vector) (Variables|Default|GetCloseDoorLocation) (Variables|Default|GetOpenDoorLocation) _alpha) false false))))

(event EventAttachVehicle
  (params (AttachSocketName :type Name :default "None"))
  (bind _workingagv (Variables|Default|GetWorkingAGV))
  (bind _returnvalue (Transformation|AttachComponentToComponent (Variables|Default|GetSupplyVehicle) (Variables|/Script/Engine.Character|GetMesh (Variables|Default|GetWorkingAGV)) AttachSocketName "SnapToTarget" "SnapToTarget" "KeepWorld" true))
  (if _returnvalue
    ;[0 0 0 0.5] AGV가 해당 차체를 참조하게끔 설정
    (bind _output_get (Variables|/Script/DigitalFactory.DFAGV|SetAttachVehicle _workingagv (Variables|Default|GetSupplyVehicle)))
    ;[0 0 0 0.5] Vehicle 색상 저장
    (Variables|/Script/DigitalFactory.DFVehicleBase|SetColor _output_get (Variables|/Script/DigitalFactory.DFAGV|GetOrderColor _workingagv))
    (Class|DFSupplyCell|InitCellData)))

(fn ConstructionScript)